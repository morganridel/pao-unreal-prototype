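; Power-up pickup actor that grants a power-up to the rolling ball when it overlaps.
; An OnBeginOverlap function, not defined in this graph, reports whether the power-up was given.
; On success it shows the power-up widget on RollingBall_BP, then hides the pickup and disables its collision.
; After a short delay the pickup reappears with collision restored, so it respawns without being destroyed.
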(event EventBeginPlay)

(event Collision|EventActorBeginOverlap
  (params (OtherActor :type Actor%20Object%20Reference))
  (bind _output_get (Variables|Default|SetOverlapping%20actor OtherActor))
  (bind _returnvalue (Class|PowerUpPickup|OnBeginOverlap _output_get))
  (if _returnvalue ; If Ball was given power up
    (Utilities|FlowControl|Sequence
      (:then_0
        (bind _asrolling_ball_bp (Utilities|Casting|CastToRollingBall_BP (Variables|Default|GetOverlapping%20actor)))
        (Widget|SetVisibility (Variables|/Game/RollingBall_BP.RollingBall_BP_C|GetPower%20Up%20Widget _asrolling_ball_bp) "Visible"))
      (:then_1
        (Rendering|SetActorHiddenInGame true)
        (Collision|SetActorEnableCollision false)
        (Utilities|FlowControl|Delay 5.0)
        (Rendering|SetActorHiddenInGame false)
        (Collision|SetActorEnableCollision true)))))

(event EventTick
  (params (DeltaSeconds :type Float%20%28single-precision%29)))

(fn ConstructionScript)