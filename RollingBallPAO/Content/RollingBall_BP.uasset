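; Player-controlled rolling ball that moves on axis input, carries usable power-ups and completes the level on reaching its end.
; Input feeds inherited roll and power-up calls, while the camera axis yaws the spring arm.
; BeginPlay binds power-up events that show or hide a HUD widget, created hidden.
; Overlapping EndLevel_BP opens the LevelSuccess widget with UI-only input and a visible cursor.
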(event EventBeginPlay
  (|BindPowerUpEvents)
  (Class|RollingBall|SetBall (Variables|Default|GetRollingBall))
  (bind _returnvalue (UserInterface|CreateWidget "/Game/UI/PowerUpDisplay.PowerUpDisplay_C"))
  (bind _output_get (Variables|Default|SetPower%20Up%20Widget _returnvalue))
  (UserInterface|Viewport|AddtoViewport _output_get 0)
  (Widget|SetVisibility _output_get "Hidden"))

(event Collision|EventActorBeginOverlap
  (params (OtherActor :type Actor%20Object%20Reference))
  (bind _returnvalue (Game|GetPlayerController 0))
  (Utilities|Casting|CastToEndLevel_BP OtherActor)
  (Development|PrintString "Overlap!")
  (bind _returnvalue_2 (UserInterface|CreateWidget "/Game/UI/LevelSuccess.LevelSuccess_C"))
  (UserInterface|Viewport|AddtoViewport _returnvalue_2 0)
  (Input|SetInputModeUIOnly _returnvalue 0 "DoNotLock")
  (Variables|/Script/Engine.PlayerController|SetbShowMouseCursor _returnvalue true))

(event Input|ActionEvents|InputActionUsePowerUp
  (params (Key :type Key%20Structure))
  (:Pressed
    (Class|RollingBall|UsePowerUp)))

(event Input|AxisEvents|InputAxisForward
  (params (AxisValue :type Float%20%28single-precision%29))
  ;[1 1 1] Movement binding
  (Class|RollingBall|RollForward AxisValue))

(event Input|AxisEvents|InputAxisCameraXRotation
  (params (AxisValue :type Float%20%28single-precision%29))
  (Transformation|AddRelativeRotation (Variables|Default|GetSpringArm) (Math|Rotator|MakeRotator 0.0 0.0 AxisValue) false false))

(event Input|AxisEvents|InputAxisRight
  (params (AxisValue :type Float%20%28single-precision%29))
  ;[1 1 1] Movement binding
  (Class|RollingBall|RollRight AxisValue))

(fn ConstructionScript)

(event Custom|OnRemovedPowerUp_Event
  (Widget|SetVisibility (Variables|Default|GetPower%20Up%20Widget) "Hidden"))

(event Custom|OnNewPowerUp_Event
  (Widget|SetVisibility (Variables|Default|GetPower%20Up%20Widget) "Visible"))